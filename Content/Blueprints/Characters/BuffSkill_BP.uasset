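; BuffSkill_BP is a temporary speed buff actor that boosts the player's walk speed and mesh animation rate while it exists.
; BeginPlay finds the player, applies the boost and calls SkillButtonTrigger on the player controller.
; After a short delay it reverts the boost, clears IsBuffOn and destroys itself.
; Tick keeps it on the player and computes a camera direction, whose rotation step is disconnected, like other leftover thunder and collision logic.
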(event OnInputTouchEnter(BuffSkill)
  (params (FingerIndex :type ETouchIndex%20Enum :default "Touch1") (TouchedComponent :type Primitive%20Component%20Object%20Reference)))

(event OnInputTouchBegin(BuffEffect)
  (params (FingerIndex :type ETouchIndex%20Enum :default "Touch1") (TouchedComponent :type Primitive%20Component%20Object%20Reference)))

(event OnInputTouchEnter(Cube)
  (params (FingerIndex :type ETouchIndex%20Enum :default "Touch1") (TouchedComponent :type Primitive%20Component%20Object%20Reference)))

(event OnComponentHit(BuffSkill)
  (params (HitComponent :type Primitive%20Component%20Object%20Reference) (OtherActor :type Actor%20Object%20Reference) (OtherComp :type Primitive%20Component%20Object%20Reference) (NormalImpulse :type Vector :default "0, 0, 0") (Hit :type Hit%20Result%20Structure%20%28by%20ref%29)))

(event OnInputTouchBegin(Cube)
  (params (FingerIndex :type ETouchIndex%20Enum :default "Touch1") (TouchedComponent :type Primitive%20Component%20Object%20Reference)))

(event OnInputTouchLeave(Cube)
  (params (FingerIndex :type ETouchIndex%20Enum :default "Touch1") (TouchedComponent :type Primitive%20Component%20Object%20Reference)))

(event OnComponentHit(BuffEffect)
  (params (HitComponent :type Primitive%20Component%20Object%20Reference) (OtherActor :type Actor%20Object%20Reference) (OtherComp :type Primitive%20Component%20Object%20Reference) (NormalImpulse :type Vector :default "0, 0, 0") (Hit :type Hit%20Result%20Structure%20%28by%20ref%29)))

(event OnInputTouchBegin(BuffSkill)
  (params (FingerIndex :type ETouchIndex%20Enum :default "Touch1") (TouchedComponent :type Primitive%20Component%20Object%20Reference)))

(event OnInputTouchEnter(BuffEffect)
  (params (FingerIndex :type ETouchIndex%20Enum :default "Touch1") (TouchedComponent :type Primitive%20Component%20Object%20Reference)))

(event EventBeginPlay
  (Utilities|FlowControl|Sequence
    (:then_0
      (bind _outactors (Actor|GetAllActorsOfClass "/Game/Blueprints/Characters/PlayerCharacters/PlayerTest_BP0.PlayerTest_BP0_C"))
      (bind _output_get (Variables|Default|SetPlayerCharacter (Utilities|Array|Get(acopy) _outactors)))
      (Variables|/Script/Engine.CharacterMovementComponent|SetMaxWalkSpeed (Variables|/Script/Engine.Character|GetCharacterMovement (Variables|Default|GetPlayerCharacter)) (* (Variables|/Script/Engine.CharacterMovementComponent|GetMaxWalkSpeed (Variables|/Script/Engine.Character|GetCharacterMovement (Variables|Default|GetPlayerCharacter))) 3.0))
      (Components|Timeline|SetPlayRate (Variables|/Script/Engine.Character|GetMesh (Variables|Default|GetPlayerCharacter)) 2.0))
    (:then_1
      (bind _outactors_2 (Actor|GetAllActorsOfClass "/Game/Blueprints/Characters/PlayerCharacters/LopolProjectPlayerController_BP.LopolProjectPlayerController_BP_C")))
    (:then_2
      (bind _outactors_3 (Actor|GetAllActorsOfClass "/Game/Blueprints/Characters/EnemyCharacters/EnemyTestBP0/EnemyTestBP0.EnemyTestBP0_C")))
    (:then_3
      (bind _outactors_4 (Actor|GetAllActorsOfClass "/Game/Blueprints/Characters/PlayerCharacters/ETC/CameraBP0.CameraBP0_C")))
    (:then_4
      (Variables|Default|SetSkillButtonExistence true)
      (Variables|Default|SetIsActivated? true))
    (:then_5
      (Default|SkillButtonTrigger (Utilities|Array|Get(acopy) _outactors_2))
      (Utilities|FlowControl|Delay 3.0)
      (Variables|Default|SetIsActivated? false)
      (Variables|/Script/Engine.CharacterMovementComponent|SetMaxWalkSpeed (Variables|/Script/Engine.Character|GetCharacterMovement (Variables|Default|GetPlayerCharacter)) (/ (Variables|/Script/Engine.CharacterMovementComponent|GetMaxWalkSpeed (Variables|/Script/Engine.Character|GetCharacterMovement (Variables|Default|GetPlayerCharacter))) 3.0))
      (Variables|/Game/Blueprints/Characters/PlayerCharacters/PlayerTest_BP0.PlayerTest_BP0_C|SetIsBuffOn? (Variables|Default|GetPlayerCharacter) false)
      (Components|Timeline|SetPlayRate (Variables|/Script/Engine.Character|GetMesh (Variables|Default|GetPlayerCharacter)) 1.0)
      (Actor|DestroyActor))))

(event Collision|EventActorBeginOverlap
  (params (OtherActor :type Actor%20Object%20Reference)))

(event EventTick
  (params (DeltaSeconds :type Float%20%28single-precision%29))
  (Utilities|FlowControl|Sequence
    (:then_0
      (Transformation|SetActorLocation (Transformation|GetActorLocation (Variables|Default|GetPlayerCharacter)) false false))
    (:then_1
      (bind _output_get (Variables|Default|SetButtonToCameraVector (Math|Vector|GetUnitDirection(Vector) (Transformation|GetActorLocation) (Transformation|GetActorLocation (Utilities|Array|Get(acopy) (stale EventBeginPlay _outactors_4)))))))))

(fn ConstructionScript)