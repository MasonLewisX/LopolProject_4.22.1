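; Unit2_BP is a character that performs a leaping attack toward an enemy location and deals damage on sphere overlap.
; LeapAttack faces the target, launches in an arc under raised gravity, then plays landing effects after a fixed delay and restores animation and gravity.
; The first sphere overlap applies damage and registers a randomized, crit-capable damage message.
; The one-shot damage flag is never reset here.
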(event OnComponentBeginOverlap(Sphere)
  (params (OverlappedComponent :type Primitive%20Component%20Object%20Reference) (OtherActor :type Actor%20Object%20Reference) (OtherComp :type Primitive%20Component%20Object%20Reference) (OtherBodyIndex :type Integer) (bFromSweep :type Boolean) (SweepResult :type Hit%20Result%20Structure%20%28by%20ref%29))
  ;[1 1 1] 데미지 적용 세트
  (if (not (Variables|Default|GetIsDamageOccured?))
    (Game|Damage|ApplyDamage 0 0.0 (Pawn|GetController (Variables|Default|GetInstigator)) self)
    (Variables|Default|SetIsDamageOccured? true)
    (Class|BPIDamageSystem|RegisterDamage(Message) OtherActor 1e+01 0.8 1.2 2e+01 2.0)))

(event Custom|LeapAttack
  (params (EnemyLocation :type Vector))
  (bind _returnvalue (Transformation|GetActorLocation))
  (bind _returnvalue_2 (Transformation|GetActorLocation))
  (bind _returnvalue_3 (- EnemyLocation _returnvalue_2))
  (bind (_x _y) (Math|Vector|BreakVector _returnvalue))
  (Variables|/Script/Engine.CharacterMovementComponent|SetGravityScale (Variables|Character|GetCharacterMovement) 3.0)
  (if (not (Variables|Default|GetIsFalling?))
    (Transformation|SetActorRotation (Math|Rotator|MakeRotationfromAxes _returnvalue_3 "0, 0, 0" "0, 0, 0"))
    (Character|LaunchCharacter (+ (/ _returnvalue_3 1.567) "0, 0,1800.000000") false true)
    (Components|Animation|PlayAnimation (Variables|Character|GetMesh) "/Game/Blueprints/Characters/PlayerCharacters/Animations/Player_Jump_Weapon.Player_Jump_Weapon" false)
    (Audio|PlaySoundatLocation 0 (Transformation|GetActorLocation) "0, 0, 0" 1.0 1.0 0.0 0 0 0)
    (Utilities|FlowControl|Delay 1.5)
    (Effects|SpawnEmitteratLocation 0 (Math|Vector|MakeVector _x _y (.Z (Math|Vector|BreakVector (Transformation|GetWorldLocation (Variables|Default|GetArrow1))))))
    (Audio|PlaySoundatLocation 0 (Transformation|GetActorLocation) "0, 0, 0" 1.0 1.0 0.0 0 0 0)
    (Components|Animation|SetAnimationMode (Variables|Character|GetMesh) "AnimationBlueprint")
    (Variables|/Script/Engine.CharacterMovementComponent|SetGravityScale (Variables|Character|GetCharacterMovement) 2.0)))

(event EventBeginPlay
  (Variables|Default|SetStartLocation (Transformation|GetActorLocation)))

(event EventTick
  (params (DeltaSeconds :type Float%20%28single-precision%29))
  (Variables|Default|SetIsFalling? (AI|Components|NavMovement|IsFalling (Pawn|GetMovementComponent))))

(event Collision|EventActorBeginOverlap
  (params (OtherActor :type Actor%20Object%20Reference)))

(fn ConstructionScript)