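; Unit1 combat character with three targeted attacks: a gravity-boosted leap, a flat rush and a burning chair throw.
; Each attack turns toward the given enemy location, then launches the character with animation and sound or spawns a FlamingChair at DropLocation.
; Hand collision overlaps, gated by per-hand flags, apply zero base damage and pass damage and crit values through RegisterDamageMessage.
; AttackRange overlaps collect LopolEnemyCharacter actors into an array.
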(event OnComponentHit(Mesh)
  (params (HitComponent :type Primitive%20Component%20Object%20Reference) (OtherActor :type Actor%20Object%20Reference) (OtherComp :type Primitive%20Component%20Object%20Reference) (NormalImpulse :type Vector :default "0, 0, 0") (Hit :type Hit%20Result%20Structure%20%28by%20ref%29)))

(event OnComponentBeginOverlap(Mesh)
  (params (OverlappedComponent :type Primitive%20Component%20Object%20Reference) (OtherActor :type Actor%20Object%20Reference) (OtherComp :type Primitive%20Component%20Object%20Reference) (OtherBodyIndex :type Integer) (bFromSweep :type Boolean) (SweepResult :type Hit%20Result%20Structure%20%28by%20ref%29)))

(event OnComponentBeginOverlap(LeftHandCollision)
  (params (OverlappedComponent :type Primitive%20Component%20Object%20Reference) (OtherActor :type Actor%20Object%20Reference) (OtherComp :type Primitive%20Component%20Object%20Reference) (OtherBodyIndex :type Integer) (bFromSweep :type Boolean) (SweepResult :type Hit%20Result%20Structure%20%28by%20ref%29))
  ;[1 1 1] 데미지 적용 세트
  (if (not (Variables|Default|GetIsLeftHandDamageOccured?))
    (Game|Damage|ApplyDamage OtherActor 0.0 (Pawn|GetController (Variables|Default|GetInstigator)) self)
    (Class|BPIDamageSystem|RegisterDamage(Message) OtherActor (Variables|Default|GetDamage) (Variables|Default|GetMinDamageModifier) (Variables|Default|GetMaxDamageModifier) (Variables|Default|GetCritChance) (Variables|Default|GetCritDamageModifier))))

(event OnComponentBeginOverlap(AttackRange)
  (params (OverlappedComponent :type Primitive%20Component%20Object%20Reference) (OtherActor :type Actor%20Object%20Reference) (OtherComp :type Primitive%20Component%20Object%20Reference) (OtherBodyIndex :type Integer) (bFromSweep :type Boolean) (SweepResult :type Hit%20Result%20Structure%20%28by%20ref%29))
  (bind _aslopol_enemy_character (Utilities|Casting|CastToLopolEnemyCharacter OtherActor))
  (bind _returnvalue (Utilities|Array|Add (Variables|Default|GetEnemyCharacter) _aslopol_enemy_character)))

(event OnComponentBeginOverlap(RightHandCollision)
  (params (OverlappedComponent :type Primitive%20Component%20Object%20Reference) (OtherActor :type Actor%20Object%20Reference) (OtherComp :type Primitive%20Component%20Object%20Reference) (OtherBodyIndex :type Integer) (bFromSweep :type Boolean) (SweepResult :type Hit%20Result%20Structure%20%28by%20ref%29))
  ;[1 1 1] 데미지 적용 세트
  (if (not (Variables|Default|GetIsRightHandDamageOccured?))
    (Game|Damage|ApplyDamage OtherActor 0.0 (Pawn|GetController (Variables|Default|GetInstigator)) self)
    (Class|BPIDamageSystem|RegisterDamage(Message) OtherActor (Variables|Default|GetDamage) (Variables|Default|GetMinDamageModifier) (Variables|Default|GetMaxDamageModifier) (Variables|Default|GetCritChance) (Variables|Default|GetCritDamageModifier))))

(event OnComponentHit(AttackCollision_R)
  (params (HitComponent :type Primitive%20Component%20Object%20Reference) (OtherActor :type Actor%20Object%20Reference) (OtherComp :type Primitive%20Component%20Object%20Reference) (NormalImpulse :type Vector :default "0, 0, 0") (Hit :type Hit%20Result%20Structure%20%28by%20ref%29)))

(event OnComponentBeginOverlap(AttackCollision_R)
  (params (OverlappedComponent :type Primitive%20Component%20Object%20Reference) (OtherActor :type Actor%20Object%20Reference) (OtherComp :type Primitive%20Component%20Object%20Reference) (OtherBodyIndex :type Integer) (bFromSweep :type Boolean) (SweepResult :type Hit%20Result%20Structure%20%28by%20ref%29)))

(event OnComponentBeginOverlap(AttackCollision_L)
  (params (OverlappedComponent :type Primitive%20Component%20Object%20Reference) (OtherActor :type Actor%20Object%20Reference) (OtherComp :type Primitive%20Component%20Object%20Reference) (OtherBodyIndex :type Integer) (bFromSweep :type Boolean) (SweepResult :type Hit%20Result%20Structure%20%28by%20ref%29)))

(event Custom|LeapAttack
  (params (EnemyLocation :type Vector))
  (bind _returnvalue (Transformation|GetActorLocation))
  (bind _returnvalue_2 (Transformation|GetActorLocation))
  (bind (_x _y) (Math|Vector|BreakVector _returnvalue))
  (bind _returnvalue_3 (- EnemyLocation _returnvalue_2))
  (Variables|/Script/Engine.CharacterMovementComponent|SetGravityScale (Variables|Character|GetCharacterMovement) 3.0)
  (if (not (Variables|Default|GetIsFalling?))
    (Transformation|SetActorRotation (Math|Rotator|MakeRotationfromAxes _returnvalue_3 "0, 0, 0" "0, 0, 0"))
    (Character|LaunchCharacter (+ (/ _returnvalue_3 1.567) "0, 0,1800.000000") false true)
    (Components|Animation|PlayAnimation (Variables|Character|GetMesh) 0 false)
    (Audio|PlaySoundatLocation 0 (Transformation|GetActorLocation) "0, 0, 0" 1.0 1.0 0.0 0 0 0)
    (Utilities|FlowControl|Delay 1.5)
    (Effects|SpawnEmitteratLocation 0 (Math|Vector|MakeVector _x _y (.Z (Math|Vector|BreakVector (Transformation|GetWorldLocation (Variables|Default|GetArrow1))))))
    (Audio|PlaySoundatLocation 0 (Transformation|GetActorLocation) "0, 0, 0" 1.0 1.0 0.0 0 0 0)
    (Components|Animation|SetAnimationMode (Variables|Character|GetMesh) "AnimationBlueprint")
    (Variables|/Script/Engine.CharacterMovementComponent|SetGravityScale (Variables|Character|GetCharacterMovement) 2.0)))

(event Custom|ThrowBurningChair
  (params (EnemyLocation :type Vector))
  (CallFunction|BurningChair EnemyLocation))

(event Custom|RushAttack
  (params (EnemyLocation :type Vector) (CharacterReferenceInput :type Lopol%20Project%20Character%20Object%20Reference))
  (bind (_x _y) (Math|Vector|BreakVector EnemyLocation))
  (bind _returnvalue (Transformation|GetActorLocation))
  (bind (_x_2 _y_2) (Math|Vector|BreakVector _returnvalue))
  (bind _returnvalue_2 (Math|Vector|MakeVector _x _y 0.0))
  (bind _returnvalue_3 (Math|Vector|MakeVector _x_2 _y_2 0.0))
  (bind _returnvalue_4 (- _returnvalue_2 _returnvalue_3))
  (bind _returnvalue_5 (* _returnvalue_4 1e+01))
  (bind (_x_3 _y_3) (Math|Vector|BreakVector _returnvalue_5))
  (Transformation|SetActorRotation (Math|Rotator|MakeRotationfromAxes _returnvalue_4 "0, 0, 0" "0, 0, 0"))
  (Components|Animation|PlayAnimation (Variables|Character|GetMesh) "/Game/Blueprints/Characters/Unit1/Animations/Unit1_RushAttack.Unit1_RushAttack" false)
  (Character|LaunchCharacter (Math|Vector|MakeVector _x_3 _y_3 0.0) false false)
  (Variables|Default|SetIsDamageOccured? false)
  (Audio|PlaySoundatLocation 0 _returnvalue "0, 0, 0" 1.0 1.0 0.0 0 0 0)
  (Components|Animation|SetAnimationMode (Variables|Character|GetMesh) "AnimationBlueprint"))

(event EventBeginPlay
  (Variables|Default|SetStartLocation (Transformation|GetActorLocation))
  (Utilities|FlowControl|Sequence
    (:then_0
      (Variables|Default|SetIsDamageOccured? true)
      (Variables|Default|SetIsLeftHandDamageOccured? true)
      (Variables|Default|SetIsRightHandDamageOccured? true))
    (:then_1
      (Components|Activation|Deactivate (Variables|Default|GetRightHandCollision)))
    (:then_2
      (Components|Activation|Deactivate (Variables|Default|GetLeftHandCollision)))))

(event EventTick
  (params (DeltaSeconds :type Float%20%28single-precision%29))
  (Variables|Default|SetIsFalling? (AI|Components|NavMovement|IsFalling (Pawn|GetMovementComponent)))
  (Utilities|FlowControl|Sequence))

(event Collision|EventActorBeginOverlap
  (params (OtherActor :type Actor%20Object%20Reference)))

(fn ConstructionScript)

(fn BurningChair
  (params (EnemyLocation :type Vector))
  (bind (_x _y) (Math|Vector|BreakVector EnemyLocation))
  (bind _returnvalue (Transformation|GetActorLocation))
  (bind _droplocation (Variables|Default|GetDropLocation))
  (bind (_x_2 _y_2) (Math|Vector|BreakVector _returnvalue))
  (bind _returnvalue_2 (Transformation|GetWorldRotation _droplocation))
  (Transformation|SetActorRotation (Math|Rotator|MakeRotationfromAxes (- (Math|Vector|MakeVector _x _y 0.0) (Math|Vector|MakeVector _x_2 _y_2 0.0)) "0, 0, 0" "0, 0, 0"))
  (Game|SpawnActorfromClass "/Game/Blueprints/Characters/PlayerCharacters/ETC/FlamingChair.FlamingChair_C" (Math|Transform|MakeTransform (+ (Transformation|GetWorldLocation _droplocation) (Math|Vector|RotateVector "0, 0, 0" _returnvalue_2)) _returnvalue_2) "Undefined" 0 0))